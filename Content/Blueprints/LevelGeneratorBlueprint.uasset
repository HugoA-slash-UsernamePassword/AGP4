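; Level generator actor that initializes a level from a random seed and then runs spawn room checks.
; On BeginPlay the server picks the seed, and Tick counts past a short frame delay before calling Initialize with it once.
; Every later tick calls CheckSpawnRoom; neither that function nor Initialize is defined in this graph.
; The Room function and the RepNotify handlers for Seed and Stream are empty.
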(event `self.ReceiveBeginPlay`
  (if (`KismetSystemLibrary.IsServer`)
    (set `self.Seed` (`KismetMathLibrary.RandomInteger` 999999))))

(event `self.ReceiveTick`
  (params (DeltaSeconds :type "Float (single-precision)"))
  (bind _result (`/Engine/EditorBlueprintResources/StandardMacros.IncrementInt` (`self.waitorsomething`))
    (:`  `
      (if (> _result 40)
        (if (`self.Initialized`)
          (`self.CheckSpawnRoom`)
          (else
            (`self.Initialize` (`self.Seed`))
            (set `self.Initialized` true)))))))

(fn `OnRep_Seed`)

(fn `OnRep_Stream`)

(fn `Room`)

(fn `UserConstructionScript`)